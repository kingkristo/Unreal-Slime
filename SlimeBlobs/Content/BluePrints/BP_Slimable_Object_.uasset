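; BP_Slimable_Object is an actor that can be slimed, provided its mesh uses a slimable material.
; On BeginPlay it creates per-instance dynamic materials and render targets, so multiple objects can coexist, unlike the floor setup.
; A SceneCapture2D showing only this actor feeds the Unwrap target into an M_Slime_Object_Intersect instance.
; A black-cleared Hit target feeds the object's own material; drawing into it happens outside this graph.
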(event Collision|EventActorBeginOverlap
  (params (OtherActor :type Actor%20Object%20Reference)))

(event EventBeginPlay
  (bind _object (Variables|Components|GetObject))
  ;[1 1 1] Note this will only work if the object is using a slimable material
  (bind _returnvalue (Rendering|Material|CreateDynamicMaterialInstance _object 0 (Utilities|Array|Get(acopy) (Rendering|Material|GetMaterials _object)) "None" :!class /Script/Engine.PrimitiveComponent))
  (Variables|Default|SetMatInstance_original _returnvalue)
  ;[1 1 1] Create dynamic render materials and set the relevant params. Unlike the floor, objects use this dynamic method to allow multiple slimable objects to be created with no issue.
  (bind _returnvalue_2 (Rendering|Material|CreateDynamicMaterialInstance "/SlimeBlobs/Materials/Slimable_Object_Materials/M_Slime_Object_Intersect.M_Slime_Object_Intersect" "None" :!class /Script/Engine.KismetMaterialLibrary))
  (Variables|Default|SetMatInstance_Hit _returnvalue_2)
  (bind _returnvalue_3 (Rendering|CreateRenderTarget2D 1024 1024 "RTF_RGBA16f"))
  (bind _output_get (Variables|Default|SetRenderTexture_Unwrap _returnvalue_3))
  (Variables|/Script/Engine.SceneCaptureComponent2D|SetTextureTarget (Variables|Components|GetSceneCaptureComponent2D) _output_get)
  (Rendering|Material|SetTextureParameterValue (Variables|Default|GetMatInstance_Hit) "Unwrap" (Variables|Default|GetRenderTexture_Unwrap))
  (Rendering|SceneCapture|ShowOnlyActorComponents (Variables|Components|GetSceneCaptureComponent2D) self false)
  (bind _returnvalue_4 (Rendering|CreateRenderTarget2D 1024 1024 "RTF_RGBA16f"))
  (Variables|Default|SetRenderTexture_Hit _returnvalue_4)
  (Rendering|Material|SetTextureParameterValue (Variables|Default|GetMatInstance_original) "Hit" (Variables|Default|GetRenderTexture_Hit))
  (Rendering|ClearRenderTarget2D (Variables|Default|GetRenderTexture_Hit)))

(fn ConstructionScript)