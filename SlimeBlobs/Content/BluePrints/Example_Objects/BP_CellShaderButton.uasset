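; BP_CellShaderButton is an example pressure button that toggles a CellShader flag when an actor overlaps it.
; The overlap eases Cylinder1 down, flips the flag, and raises the cylinder again after a two-second delay, with ButtonPressed blocking retriggers meanwhile.
; A graph comment mentions moving a cel shader post-process volume toward the player, but this Blueprint contains no such movement.
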(event Collision|EventActorBeginOverlap
  (params (OtherActor :type Actor%20Object%20Reference))
  (bind _cylinder1 (Variables|Default|GetCylinder1))
  ;[1 1 1] Move cell shader post process volume towards player when button is pressed
  (if (not (Variables|Default|GetButtonPressed))
    (Components|MoveComponentTo _cylinder1 "0,0.000000,-2.000000" "0, 0, 0" true true 0.2 false)
    (Variables|Default|SetButtonPressed true)
    (Variables|Default|SetCellShader (not (Variables|Default|GetCellShader)))
    (Utilities|FlowControl|Delay 2.0)
    (Components|MoveComponentTo _cylinder1 "0,0.000000,4.000000" "0, 0, 0" true true 0.2 false)
    (Variables|Default|SetButtonPressed false)))

(fn ConstructionScript
  (Variables|Default|SetButtonPressed false))