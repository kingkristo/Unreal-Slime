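; Scene capture actor that records floor trails around the player into render targets, adapted from a snow-trail tutorial.
; Each tick it follows the player, snapped to capture-pixel size to keep texels aligned, and publishes its location and size to a material parameter collection.
; A dynamic material then draws into the persistent render target, offset by the movement.
; Trails survive long travel but are lost outside the capture area.
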(event EventBeginPlay
  ;[1 1 1] Render texture method adapted from: https://www.raywenderlich.com/5760-creating-snow-trails-in-unreal-engine-4
  (Rendering|Material|SetScalarParameterValue "/SlimeBlobs/Materials/Floor_Trail_Materials/MPC_Floor_Trail_Variables.MPC_Floor_Trail_Variables" "CaptureSize" (Variables|/Script/Engine.SceneCaptureComponent2D|GetOrthoWidth (Variables|Default|GetSceneCapture)) :!class /Script/Engine.KismetMaterialLibrary)
  (bind _returnvalue (Rendering|Material|CreateDynamicMaterialInstance "/SlimeBlobs/Materials/Floor_Trail_Materials/M_DrawToPersistentFloorRT.M_DrawToPersistentFloorRT" "None" :!class /Script/Engine.KismetMaterialLibrary))
  (Variables|Default|SetDrawMaterial _returnvalue)
  (Rendering|ClearRenderTarget2D "/SlimeBlobs/Materials/Textures/Floor_RT_Current.Floor_RT_Current")
  (Rendering|ClearRenderTarget2D "/SlimeBlobs/Materials/Textures/Floor_RT_Perminent.Floor_RT_Perminent"))

(event EventTick
  (params (DeltaSeconds :type Float%20%28single-precision%29))
  ;[1 1 1] Render texture method adapted from: https://www.raywenderlich.com/5760-creating-snow-trails-in-unreal-engine-4
  (CallFunction|MoveCapture)
  (CallFunction|DrawtoPersistent))

(fn ConstructionScript)

(fn DrawtoPersistent
  (bind _scenecapture (Variables|Default|GetSceneCapture))
  (bind _moveoffset (Variables|Default|GetMoveOffset))
  (bind _orthowidth (Variables|/Script/Engine.SceneCaptureComponent2D|GetOrthoWidth _scenecapture))
  (bind _returnvalue (/ _moveoffset _orthowidth))
  (Rendering|Material|SetVectorParameterValue (Variables|Default|GetDrawMaterial) "Offset" (Utilities|Struct|MakeLinearColor (.x _returnvalue) (.y _returnvalue) 0.0 1.0) :!class /Script/Engine.MaterialInstanceDynamic)
  (Rendering|DrawMaterialtoRenderTarget "/SlimeBlobs/Materials/Textures/Floor_RT_Perminent.Floor_RT_Perminent" (Variables|Default|GetDrawMaterial)))

(fn MoveCapture
  (bind _returnvalue (Transformation|GetActorLocation))
  (bind _returnvalue_2 (Game|GetPlayerCharacter 0))
  (bind _returnvalue_3 (/ 1.0 256.0))
  (bind _scenecapture (Variables|Default|GetSceneCapture))
  (bind _returnvalue_4 (Transformation|GetActorLocation _returnvalue_2))
  (bind _orthowidth (Variables|/Script/Engine.SceneCaptureComponent2D|GetOrthoWidth _scenecapture))
  (bind _returnvalue_5 (* _orthowidth _returnvalue_3))
  (bind _returnvalue_6 (Utilities|SnaptoPixelWorldSize (.x _returnvalue_4) (.y _returnvalue_4) _returnvalue_5))
  (bind _returnvalue_7 (- _returnvalue_6 _returnvalue))
  ;[1 1 1] Make the scene capture area follow the player, so that they can travel very far on the terrain and still leave a trail with no problem. (Downside is that the old trail will be erased if they move to far away)
  (bind _output_get (Variables|Default|SetMoveOffset (Math|Vector2D|MakeVector2D (.x _returnvalue_7) (.y _returnvalue_7))))
  (Transformation|AddActorWorldOffset (Math|Vector|MakeVector (.x _output_get) (.y _output_get) 0.0))
  (Rendering|Material|SetVectorParameterValue "/SlimeBlobs/Materials/Floor_Trail_Materials/MPC_Floor_Trail_Variables.MPC_Floor_Trail_Variables" "CaptureLocation" (Math|Conversions|ToLinearColor(Vector) (Transformation|GetActorLocation)) :!class /Script/Engine.KismetMaterialLibrary))